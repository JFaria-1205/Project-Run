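; BP_Doorway is a trigger actor that streams levels as the player passes through a doorway.
; When the player character enters its Box, it asks BP_LevelManager to spawn a new, non-first level at its Arrow's world location; leaving the Box tells the manager to despawn the old level.
; The manager is cached on BeginPlay, with a fresh actor lookup as fallback if that reference is invalid.
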(event OnComponentBeginOverlap(Box)
  (params (OverlappedComponent :type Primitive%20Component%20Object%20Reference) (OtherActor :type Actor%20Object%20Reference) (OtherComp :type Primitive%20Component%20Object%20Reference) (OtherBodyIndex :type Integer) (bFromSweep :type Boolean) (SweepResult :type Hit%20Result%20Structure%20%28by%20ref%29))
  (bind _arrow (Variables|Default|GetArrow))
  (bind _levelmanager (Variables|Default|GetLevelManager))
  (bind _returnvalue (Transformation|GetWorldLocation _arrow))
  (if (== OtherActor (Game|GetPlayerCharacter 0))
    (Utilities|IsValid _levelmanager
      (:Is%20Valid
        (Default|SpawnNewLevel _levelmanager _returnvalue false))
      (:Is%20Not%20Valid
        (bind _returnvalue_2 (Actor|GetActorOfClass "/Game/Level_Stream_Actors/BP_LevelManager.BP_LevelManager_C"))
        (Default|SpawnNewLevel _returnvalue_2 _returnvalue false)))))

(event OnComponentEndOverlap(Box)
  (params (OverlappedComponent :type Primitive%20Component%20Object%20Reference) (OtherActor :type Actor%20Object%20Reference) (OtherComp :type Primitive%20Component%20Object%20Reference) (OtherBodyIndex :type Integer))
  (bind _levelmanager (Variables|Default|GetLevelManager))
  (if (== OtherActor (Game|GetPlayerCharacter 0))
    (Utilities|IsValid _levelmanager
      (:Is%20Valid
        (Default|DespawnOldLevel _levelmanager))
      (:Is%20Not%20Valid
        (bind _returnvalue (Actor|GetActorOfClass "/Game/Level_Stream_Actors/BP_LevelManager.BP_LevelManager_C"))
        (Default|DespawnOldLevel _returnvalue)))))

(event EventBeginPlay
  (bind _returnvalue (Actor|GetActorOfClass "/Game/Level_Stream_Actors/BP_LevelManager.BP_LevelManager_C"))
  (Variables|Default|SetLevelManager _returnvalue))

(fn ConstructionScript)