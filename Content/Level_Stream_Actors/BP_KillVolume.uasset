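; Moving kill volume that kills the player when it catches up with them.
; While enabled, Tick sweeps the actor along a normalized Direction at Speed, scaled by delta time and based on the Box's world location.
; Box overlap with the player pawn calls PlayerDeath on BP_FirstPersonCharacter.
; MoveKillVolume and StopKillVolume toggle the movement; the overlap kill does not depend on it.
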(event OnComponentBeginOverlap(Box)
  (params (OverlappedComponent :type Primitive%20Component%20Object%20Reference) (OtherActor :type Actor%20Object%20Reference) (OtherComp :type Primitive%20Component%20Object%20Reference) (OtherBodyIndex :type Integer) (bFromSweep :type Boolean) (SweepResult :type Hit%20Result%20Structure%20%28by%20ref%29))
  (bind _returnvalue (Game|Player|GetPlayerPawn 0))
  ;[1 1 1] Kill player if caught up
  (if (== OtherActor _returnvalue)
    (bind _asbp_first_person_character (Utilities|Casting|CastToBP_FirstPersonCharacter _returnvalue))
    (Default|PlayerDeath _asbp_first_person_character)))

(event Custom|MoveKillVolume
  ;[1 1 1] Start/Stop moving
  (Variables|Default|Setmove? true))

(event Custom|StopKillVolume
  ;[1 1 1] Start/Stop moving
  (Variables|Default|Setmove? false))

(event EventTick
  (params (DeltaSeconds :type Float%20%28single-precision%29))
  ;[1 1 1] Constant Movement
  (if (Variables|Default|Getmove?)
    (Transformation|SetActorLocation (+ (* (Math|Vector|Normalize (Variables|Default|Getdirection)) (* (Utilities|Time|GetWorldDeltaSeconds) (Variables|Default|Getspeed))) (Transformation|GetWorldLocation (Variables|Default|GetBox))) true false)))

(fn ConstructionScript)