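; BP_LevelManager is an actor that streams level chunks in and out as runtime level instances.
; On BeginPlay it loads a fixed starting level and spawns a BP_KillVolume.
; SpawnNewLevel otherwise loads a random entry from LevelList at the given location, keeping the previous instance as OldLevel.
; DespawnOldLevel unloads that instance, moves the kill volume's box to the newest spawn location and calls MoveKillVolume.
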(event EventBeginPlay
  (CallFunction|Initialize))

(event Collision|EventActorBeginOverlap
  (params (OtherActor :type Actor%20Object%20Reference)))

(event EventTick
  (params (DeltaSeconds :type Float%20%28single-precision%29)))

(fn ConstructionScript)

(fn SpawnNewLevel
  (params (Location :type Vector) (FirstLevel :type Boolean))
  (bind _levellist (Variables|Default|GetLevelList))
  (bind _levelreferences (Utilities|Struct|BreakStruct_LevelList _levellist))
  (if FirstLevel
    ;[1 1 1] Spawn first level
    (bind _returnvalue (Class|LevelStreamingDynamic|LoadLevelInstancebySoftObjectPtr "/Game/Levels/SpawnTestLevels/LVL_Test_Spawn.LVL_Test_Spawn" "0, 0, 0" "0, 0, 0" "" 0 false))
    (Variables|Default|SetCurrentLevel _returnvalue)
    (else
      ;[1 1 1] Default Level Spawn
      (bind _output_get (Variables|Default|SetNewLevelSpawnLocation Location))
      (bind _returnvalue_2 (Class|LevelStreamingDynamic|LoadLevelInstancebySoftObjectPtr (Utilities|Struct|BreakSoftWorldReference (Utilities|Array|Get(acopy) _levelreferences (Math|Random|RandomIntegerinRange 0 (- (Utilities|Array|Length _levelreferences) 1)))) _output_get "0, 0, 0" "" 0 false))
      (Variables|Default|SetOldLevel (Variables|Default|GetCurrentLevel))
      (Variables|Default|SetCurrentLevel _returnvalue_2))))

(fn DespawnOldLevel
  (Class|LevelStreaming|SetIsRequestingUnloadandRemoval (Variables|Default|GetOldLevel) true)
  (Transformation|SetWorldLocation (Variables|/Game/Level_Stream_Actors/BP_KillVolume.BP_KillVolume_C|GetBox (Variables|Default|GetKillVolume)) (Variables|Default|GetNewLevelSpawnLocation) false false)
  (Default|MoveKillVolume (Variables|Default|GetKillVolume)))

(fn Initialize
  (CallFunction|SpawnNewLevel "0, 0, 0" true)
  (bind _returnvalue (Game|SpawnActorfromClass "/Game/Level_Stream_Actors/BP_KillVolume.BP_KillVolume_C" (Math|Transform|MakeTransform "-500.000000,0.000000,0.000000" "0, 0, 0" "1.000000,1.000000,1.000000") "Undefined" "MultiplyWithRoot" 0 0))
  (Variables|Default|SetKillVolume _returnvalue))