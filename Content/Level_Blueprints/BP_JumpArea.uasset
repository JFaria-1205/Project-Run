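; BP_JumpArea is a jump zone that grants the first-person player an extra jump while they overlap JumpArea.
; On BeginPlay it finds and caches the BP_FirstPersonCharacter through GetActorOfClass.
; Overlap begin and end events filter for that player, raise or lower JumpMaxCount by one, and print the new count for debugging.
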(event OnActorBeginOverlap(JumpArea)
  (params (OverlappedActor :type Actor%20Object%20Reference) (OtherActor :type Actor%20Object%20Reference))
  (bind _player (Variables|Default|GetPlayer))
  (if (== OtherActor (Variables|Default|GetPlayer))
    (bind _output_get (Variables|/Script/Engine.Character|SetJumpMaxCount _player (+ (Variables|/Script/Engine.Character|GetJumpMaxCount _player) 1)))
    (Development|PrintString (Utilities|String|ToString(Integer) _output_get))))

(event OnActorEndOverlap(JumpArea)
  (params (OverlappedActor :type Actor%20Object%20Reference) (OtherActor :type Actor%20Object%20Reference))
  (bind _player (Variables|Default|GetPlayer))
  (if (== OtherActor (Variables|Default|GetPlayer))
    (bind _output_get (Variables|/Script/Engine.Character|SetJumpMaxCount _player (- (Variables|/Script/Engine.Character|GetJumpMaxCount _player) 1)))
    (Development|PrintString (Utilities|String|ToString(Integer) _output_get))))

(event EventBeginPlay
  (bind _returnvalue (Actor|GetActorOfClass "/Game/UnrealStartingContent/FirstPerson/Blueprints/BP_FirstPersonCharacter.BP_FirstPersonCharacter_C"))
  (Variables|Default|SetPlayer _returnvalue))

(fn ConstructionScript)